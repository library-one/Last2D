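; A PaperZD 2D character that, despite its AI name, is driven by player Enhanced Input for horizontal movement, jumping and attacking.
; BeginPlay adds the input mapping context to player 0's subsystem, while jump, ledge-fall and attack events jump directly to nodes in the animation state machine.
; Damage only prints a debug message, and FlipTurn, which would rotate the controller to face the movement direction, is never executed.
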(event `self.ReceiveBeginPlay`
  (bind _asmy_player_controller (cast `MyPlayerController` (`GameplayStatics.GetPlayerController` 0)))
  (`EnhancedInputSubsystemInterface.AddMappingContext` (pcsubsystem `EnhancedInputLocalPlayerSubsystem` _asmy_player_controller) null 0 (struct)))

(event `EnhancedInput|/Game/Input/IA_Move`
  (params (ActionValue :type "Float (double-precision)") (ElapsedSeconds :type "Float (double-precision)") (TriggeredSeconds :type "Float (double-precision)") (InputAction :type "InputAction Object Reference" :default "/Game/Input/IA_Move.IA_Move"))
  (:`Triggered`
    (`self.AddMovementInput` (1.0 0.0 0.0) ActionValue)))

(event `EnhancedInput|/Game/Input/IA_Jump`
  (params (ActionValue :type Boolean) (ElapsedSeconds :type "Float (double-precision)") (TriggeredSeconds :type "Float (double-precision)") (InputAction :type "InputAction Object Reference" :default "/Game/Input/IA_Jump.IA_Jump"))
  (:`Triggered`
    (`self.Jump`)))

(event `self.OnJumped`
  (`PaperZDAnimInstance.JumpToNode` (`PaperZDAnimationComponent.AnimInstance` (`self.AnimationComponent`)) "JumpActivated" "None"))

(event `self.OnWalkingOffLedge`
  (params (PreviousFloorImpactNormal :type "Vector Structure (by ref)") (PreviousFloorContactNormal :type "Vector Structure (by ref)") (PreviousLocation :type "Vector Structure (by ref)") (TimeDelta :type "Float (single-precision)"))
  (`PaperZDAnimInstance.JumpToNode` (`PaperZDAnimationComponent.AnimInstance` (`self.AnimationComponent`)) "FallActive" "None"))

(event `EnhancedInput|/Game/Input/IA_Attack`
  (params (ActionValue :type Boolean) (ElapsedSeconds :type "Float (double-precision)") (TriggeredSeconds :type "Float (double-precision)") (InputAction :type "InputAction Object Reference" :default "/Game/Input/IA_Attack.IA_Attack"))
  (:`Triggered`
    (`PaperZDAnimInstance.JumpToNode` (`PaperZDAnimationComponent.AnimInstance` (`self.AnimationComponent`)) "Attackactived" "None")))

(event `self.ReceiveAnyDamage`
  (params (Damage :type "Float (single-precision)") (DamageType :type "DamageType Object Reference") (InstigatedBy :type "Controller Object Reference") (DamageCauser :type "Actor Object Reference"))
  (`KismetSystemLibrary.PrintString` (`KismetStringLibrary.Concat_StrStr` (`KismetStringLibrary.Conv_DoubleToString` Damage) (`KismetSystemLibrary.GetDisplayName` DamageType)) true true (struct :`R` 1.0 :`B` 0.318894 :`A` 1.0) 4.0))

(fn `Flip Turn`
  (params (Input :type "Float (double-precision)"))
  (bind _returnvalue (`self.GetController`))
  (`/Engine/EditorBlueprintResources/StandardMacros.CompareFloat` Input
    (:`>`
      (`Controller.SetControlRotation` _returnvalue (`KismetMathLibrary.MakeRotator` 0.0)))
    (:`<`
      (`Controller.SetControlRotation` _returnvalue (`KismetMathLibrary.MakeRotator` 0.0 0.0 180.0)))))

(fn `UserConstructionScript`)